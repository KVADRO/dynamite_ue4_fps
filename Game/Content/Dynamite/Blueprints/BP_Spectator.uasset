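; BP_Spectator is a temporary spectator pawn that holds a player through a respawn countdown.
; Possession starts the timer and creates a WBP_Spectator widget for the locally controlled player, which Tick updates with whole seconds remaining.
; At zero, the authority spawns a FirstPersonCharacter at a random PlayerStart, hands the controller over, then destroys the spectator and removes its UI.
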(event `self.ReceivePossessed`
  (params (NewController :type "Controller Object Reference"))
  (`|ExecutionSequence`
    (:`then_0`
      ;[1 1 1] Init initial timer value and activate timer
      (set `self.TimeoutCurrent` (`self.TimeoutMax`))
      (set `self.IsTimerActive` true))
    (:`then_1`
      ;[1 1 1] Create UI for local client
      (if (`self.IsLocallyControlled`)
        (bind _returnvalue (`|CreateWidget` "/Game/Dynamite/UI/WBP_Spectator.WBP_Spectator_C" (`GameplayStatics.GetPlayerController` 0)))
        (bind _output_get (set `self.SpectatorUI` _returnvalue))
        (`UserWidget.AddToViewport` _output_get 0)
        (`/Game/Dynamite/UI/WBP_Spectator.SetTimeout` _output_get (`KismetMathLibrary.FTrunc` (`self.TimeoutCurrent`)))))))

(event `self.ReceiveTick`
  (params (DeltaSeconds :type "Float (single-precision)"))
  (if (`self.IsTimerActive`)
    (`|ExecutionSequence`
      (:`then_0`
        ;[1 1 1] Update timeout
        (set `self.TimeoutCurrent` (`KismetMathLibrary.FClamp` (- (`self.TimeoutCurrent`) (`GameplayStatics.GetWorldDeltaSeconds`)) 0.0 (`self.TimeoutMax`))))
      (:`then_1`
        ;[1 1 1] Update UI
        (if (`self.IsLocallyControlled`)
          (`/Game/Dynamite/UI/WBP_Spectator.SetTimeout` (`self.SpectatorUI`) (`KismetMathLibrary.FTrunc` (`self.TimeoutCurrent`)))))
      (:`then_2`
        ;[1 1 1] Check is timer copleted
        (bind _output_get (set `self.IsTimerActive` (not (`KismetMathLibrary.NearlyEqual_FloatFloat` (`self.TimeoutCurrent`) 0.0 0.0001))))
        (if (and (not _output_get) (`self.HasAuthority`))
          (bind _output_get_2 (set `self.PC` (`self.GetController`)))
          (`Controller.UnPossess` _output_get_2)
          (bind _returnvalue (`|SpawnActorFromClass` "/Game/FirstPersonBP/Blueprints/FirstPersonCharacter.FirstPersonCharacter_C" (`self.GetSpawnTransform`) "Undefined" "OverrideRootScale" null null))
          (`Controller.Possess` (`self.PC`) _returnvalue)
          (`self.K2_DestroyActor`)
          (`Widget.RemoveFromParent` (`self.SpectatorUI`)))))))

(fn `GetSpawnTransform`
  (returns (Result :type "Transform Structure"))
  (bind _outactors (`GameplayStatics.GetAllActorsOfClass` "/Script/Engine.PlayerStart"))
  (return (`self.GetTransform` (`|GetArrayItem` _outactors (`KismetMathLibrary.RandomInteger` (`KismetArrayLibrary.Array_Length` _outactors))))))

(fn `UserConstructionScript`)