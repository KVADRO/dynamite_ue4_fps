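; Dynamite actor that explodes after a short fuse and kills the first-person characters within its blast sphere.
; On BeginPlay the server sets a lifespan as the fuse, so the explosion logic lives in EndPlay.
; EndPlay spawns the explosion particle without an authority check, while only the authority calls DynamiteKill on overlapping characters, passing their location and an unnormalized direction away from the blast.
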(event `self.ReceiveBeginPlay`
  (if (`self.HasAuthority`)
    (`self.SetLifeSpan` 3.0)))

(event `self.ReceiveEndPlay`
  (params (EndPlayReason :type "EEndPlayReason Enum" :default "Destroyed"))
  (`GameplayStatics.SpawnEmitterAtLocation` "/Game/StarterContent/Particles/P_Explosion.P_Explosion" (`self.K2_GetActorLocation`))
  ;[1 1 1] Dynamite kill
  (if (`self.HasAuthority`)
    (for _array_element (`PrimitiveComponent.GetOverlappingActors` (`self.Sphere`) "/Game/FirstPersonBP/Blueprints/FirstPersonCharacter.FirstPersonCharacter_C")
      (bind _asfirst_person_character (cast `/Game/FirstPersonBP/Blueprints/FirstPersonCharacter` _array_element))
      (bind _returnvalue (`self.K2_GetActorLocation` _asfirst_person_character))
      (`/Game/FirstPersonBP/Blueprints/FirstPersonCharacter.DynamiteKill` _asfirst_person_character _returnvalue (- _returnvalue (`self.K2_GetActorLocation`))))))

(fn `UserConstructionScript`)